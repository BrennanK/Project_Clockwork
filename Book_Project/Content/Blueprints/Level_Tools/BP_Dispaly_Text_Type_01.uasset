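; Level tool actor that shows and hides tutorial text in the player's dialogue panel.
; ShowTutorialText reads a dialogue row from an indexed array of DataTables, using a numeric index as row name, then fills BP_Avatar's UI panel and loops its press-A animation.
; HideTutorialText stops that animation and hides the panel through the stored Player reference.
; Neither event is triggered within this Blueprint.
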(event EventBeginPlay)

(event Collision|EventActorBeginOverlap
  (params (OtherActor :type Actor%20Object%20Reference)))

(event EventTick
  (params (DeltaSeconds :type Float%20%28single-precision%29)))

(event EventShowTutorialText
  (bind _returnvalue (Utilities|GetDataTableRow (Utilities|Array|Get(acopy) (Variables|Default|GetData%20Table%20Reference) (Variables|Default|GetindexOfDataTableReference)) (Utilities|String|StringToName (Utilities|String|ToString(Integer) (Variables|Default|GetindexOfDataTable))))
    (:then
      (bind _asbp_avatar (Utilities|Casting|CastToBP_Avatar (Game|GetPlayerCharacter 0)))
      (Widget|SetVisibility (Variables|/Game/Blueprints/Widgets/Player_UI.Player_UI_C|GetDialogePanel (Variables|/Game/Blueprints/Characters_NPC_S/BP_Avatar.BP_Avatar_C|GetPlayer%20UI%20Reference _asbp_avatar)) "Visible")
      (UserInterface|Animation|PlayAnimation (Variables|/Game/Blueprints/Characters_NPC_S/BP_Avatar.BP_Avatar_C|GetPlayer%20UI%20Reference _asbp_avatar) (Variables|/Game/Blueprints/Widgets/Player_UI.Player_UI_C|GetPress_A_Animation (Variables|/Game/Blueprints/Characters_NPC_S/BP_Avatar.BP_Avatar_C|GetPlayer%20UI%20Reference _asbp_avatar)) 0.0 0 "Forward" 1.0)
      (Rendering|Components|TextRender|SetText (Variables|/Game/Blueprints/Widgets/Player_UI.Player_UI_C|GetDialogueBoxText (Variables|/Game/Blueprints/Characters_NPC_S/BP_Avatar.BP_Avatar_C|GetPlayer%20UI%20Reference _asbp_avatar)) (Utilities|Struct|BreakDialogue_Struct _returnvalue)))))

(event EventHideTutorialText
  (bind _asbp_avatar (Utilities|Casting|CastToBP_Avatar (Variables|Default|Getplayer)))
  (Class|UserWidget|StopAnimation (Variables|/Game/Blueprints/Characters_NPC_S/BP_Avatar.BP_Avatar_C|GetPlayer%20UI%20Reference _asbp_avatar) (Variables|/Game/Blueprints/Widgets/Player_UI.Player_UI_C|GetPress_A_Animation (Variables|/Game/Blueprints/Characters_NPC_S/BP_Avatar.BP_Avatar_C|GetPlayer%20UI%20Reference _asbp_avatar)))
  (Widget|SetVisibility (Variables|/Game/Blueprints/Widgets/Player_UI.Player_UI_C|GetDialogePanel (Variables|/Game/Blueprints/Characters_NPC_S/BP_Avatar.BP_Avatar_C|GetPlayer%20UI%20Reference _asbp_avatar)) "Hidden"))

(fn ConstructionScript)

(fn NewFunction0)