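; Level actor that drives the player HUD's pop-up counters for fragments, time ability shards and lives.
; It caches the BP_Avatar on BeginPlay and works through its PlayerUIReference.
; Each update event plays a reveal animation, refreshes the value, then reverses it after a retriggerable delay if no other counter is showing.
; A negative LifeObtainedCount in the life update instead opens the Tutuorial_Complete widget with UI-only input.
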(event EventBeginPlay
  (bind _asbp_avatar (Utilities|Casting|CastToBP_Avatar (Game|GetPlayerCharacter 0))
    (:then
      (Variables|Default|SetPlayer _asbp_avatar))
    (:CastFailed
      (Development|PrintString "Kill me"))))

(event Collision|EventActorBeginOverlap
  (params (OtherActor :type Actor%20Object%20Reference)))

(event EventTick
  (params (DeltaSeconds :type Float%20%28single-precision%29)))

(event EventUpdateFragmentCount
  (params (shardWorth :type Integer))
  (bind _player (Variables|Default|GetPlayer))
  (bind _player_2 (Variables|Default|GetPlayer))
  (bind _player_ui_reference (Variables|/Game/Blueprints/Characters_NPC_S/BP_Avatar.BP_Avatar_C|GetPlayer%20UI%20Reference _player))
  (bind _player_ui_reference_2 (Variables|/Game/Blueprints/Characters_NPC_S/BP_Avatar.BP_Avatar_C|GetPlayer%20UI%20Reference _player_2))
  (bind _frag_count_display (Variables|/Game/Blueprints/Widgets/Player_UI.Player_UI_C|GetFrag_Count_Display _player_ui_reference))
  (if (Variables|/Game/Blueprints/Widgets/Player_UI.Player_UI_C|GetFrag_Count_Showing _player_ui_reference)
    _
    (else
      (Variables|/Game/Blueprints/Widgets/Player_UI.Player_UI_C|SetFrag_Count_Showing _player_ui_reference true)
      (UserInterface|Animation|PlayAnimation _player_ui_reference _frag_count_display 0.0 1 "Forward" 1.0)
      (Utilities|FlowControl|Delay (Class|WidgetAnimation|GetEndTime _frag_count_display))))
  (Default|UpdateDFrag _player_ui_reference)
  (if (Variables|/Game/Blueprints/Widgets/Player_UI.Player_UI_C|GetFrag_Count_Showing _player_ui_reference_2)
    (if (not (Variables|/Game/Blueprints/Widgets/Player_UI.Player_UI_C|GetLife_Count_Showing _player_ui_reference_2))
      (if (not (Variables|/Game/Blueprints/Widgets/Player_UI.Player_UI_C|GetTime_Shard_Showing _player_ui_reference_2))
        (Utilities|FlowControl|RetriggerableDelay 0.5)
        (UserInterface|Animation|PlayAnimation _player_ui_reference_2 (Variables|/Game/Blueprints/Widgets/Player_UI.Player_UI_C|GetFrag_Count_Display _player_ui_reference_2) 0.0 1 "Reverse" 1.0)
        (Variables|/Game/Blueprints/Widgets/Player_UI.Player_UI_C|SetFrag_Count_Showing _player_ui_reference_2 false)))))

(event EventUpdateAbilityShardCount
  (bind _player (Variables|Default|GetPlayer))
  (bind _player_2 (Variables|Default|GetPlayer))
  (bind _player_ui_reference (Variables|/Game/Blueprints/Characters_NPC_S/BP_Avatar.BP_Avatar_C|GetPlayer%20UI%20Reference _player))
  (bind _player_ui_reference_2 (Variables|/Game/Blueprints/Characters_NPC_S/BP_Avatar.BP_Avatar_C|GetPlayer%20UI%20Reference _player_2))
  (bind _time_ability_shard_count (Variables|/Game/Blueprints/Widgets/Player_UI.Player_UI_C|GetTime_Ability_Shard_Count _player_ui_reference))
  (if (Variables|/Game/Blueprints/Widgets/Player_UI.Player_UI_C|GetTime_Shard_Showing _player_ui_reference)
    _
    (else
      (Variables|/Game/Blueprints/Widgets/Player_UI.Player_UI_C|SetTime_Shard_Showing _player_ui_reference true)
      (UserInterface|Animation|PlayAnimation _player_ui_reference _time_ability_shard_count 0.0 1 "Forward" 1.0)
      (Utilities|FlowControl|Delay (Class|WidgetAnimation|GetEndTime _time_ability_shard_count))))
  (Default|UpdateTACount _player_ui_reference)
  (if (not (Variables|/Game/Blueprints/Widgets/Player_UI.Player_UI_C|GetFrag_Count_Showing _player_ui_reference_2))
    (if (not (Variables|/Game/Blueprints/Widgets/Player_UI.Player_UI_C|GetLife_Count_Showing _player_ui_reference_2))
      (if (Variables|/Game/Blueprints/Widgets/Player_UI.Player_UI_C|GetTime_Shard_Showing _player_ui_reference_2)
        (Utilities|FlowControl|RetriggerableDelay 0.5)
        (UserInterface|Animation|PlayAnimation _player_ui_reference_2 (Variables|/Game/Blueprints/Widgets/Player_UI.Player_UI_C|GetTime_Ability_Shard_Count _player_ui_reference_2) 0.0 1 "Reverse" 1.0)
        (Variables|/Game/Blueprints/Widgets/Player_UI.Player_UI_C|SetTime_Shard_Showing _player_ui_reference_2 false)))))

(event EventUpdateLifeCount
  (bind _player (Variables|Default|GetPlayer))
  (bind _player_2 (Variables|Default|GetPlayer))
  (bind _player_ui_reference (Variables|/Game/Blueprints/Characters_NPC_S/BP_Avatar.BP_Avatar_C|GetPlayer%20UI%20Reference _player))
  (bind _player_ui_reference_2 (Variables|/Game/Blueprints/Characters_NPC_S/BP_Avatar.BP_Avatar_C|GetPlayer%20UI%20Reference _player_2))
  (bind _life_count (Variables|/Game/Blueprints/Widgets/Player_UI.Player_UI_C|GetLife_Count _player_ui_reference_2))
  (if (< (Variables|Default|GetLife_Obtained_Count) 0)
    (bind _returnvalue (UserInterface|CreateWidget "/Game/Blueprints/Widgets/Tutuorial_Complete.Tutuorial_Complete_C"))
    (UserInterface|Viewport|AddtoViewport _returnvalue 0)
    (Input|SetInputModeUIOnly (Game|GetPlayerController 0) 0 "DoNotLock")
    (else
      (if (Variables|/Game/Blueprints/Widgets/Player_UI.Player_UI_C|GetLife_Count_Showing _player_ui_reference_2)
        _
        (else
          (Variables|/Game/Blueprints/Widgets/Player_UI.Player_UI_C|SetLife_Count_Showing _player_ui_reference_2 true)
          (UserInterface|Animation|PlayAnimation _player_ui_reference_2 _life_count 0.0 1 "Forward" 1.0)
          (Utilities|FlowControl|Delay (Class|WidgetAnimation|GetEndTime _life_count))))
      (Default|UpdateLives _player_ui_reference_2)
      (if (not (Variables|/Game/Blueprints/Widgets/Player_UI.Player_UI_C|GetFrag_Count_Showing _player_ui_reference))
        (if (Variables|/Game/Blueprints/Widgets/Player_UI.Player_UI_C|GetLife_Count_Showing _player_ui_reference)
          (if (not (Variables|/Game/Blueprints/Widgets/Player_UI.Player_UI_C|GetTime_Shard_Showing _player_ui_reference))
            (Utilities|FlowControl|RetriggerableDelay 0.5)
            (UserInterface|Animation|PlayAnimation _player_ui_reference (Variables|/Game/Blueprints/Widgets/Player_UI.Player_UI_C|GetLife_Count _player_ui_reference) 0.0 1 "Reverse" 1.0)
            (Variables|/Game/Blueprints/Widgets/Player_UI.Player_UI_C|SetLife_Count_Showing _player_ui_reference false)))))))

(fn ConstructionScript)