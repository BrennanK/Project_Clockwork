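; AI controller for patrolling enemies that feeds patrol and player-detection state into the blackboard.
; On BeginPlay it casts its pawn to BP_Patrolling_Enemy, copies the patrol path's looping flag and wait time, and sets an initial direction.
; AI Perception updates CanSeePlayer with the sensed result whenever the stimulus actor is a BP_Avatar.
; A debug message prints on each such update, including when sight is lost.
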(event OnTargetPerceptionUpdated(AIPerception)
  (params (Actor :type Actor%20Object%20Reference) (Stimulus :type AI%20Stimulus%20Structure))
  (Utilities|Casting|CastToBP_Avatar Actor)
  (AI|Components|Blackboard|SetValueasBool (AI|GetBlackboard 0) (Utilities|Name|MakeLiteralName "CanSeePlayer") (.bSuccessfullySensed (Utilities|Struct|BreakAIStimulus Stimulus)))
  (Development|PrintString "Found player via stimulus" true true "(R=0.000000,G=0.660000,B=1.000000,A=1.000000)" 6.0))

(event EventBeginPlay
  (bind _returnvalue (AI|GetBlackboard 0))
  (bind _asbp_patrolling_enemy (Utilities|Casting|CastToBP_Patrolling_Enemy (Pawn|GetControlledPawn)))
  (bind _output_get (Variables|Default|SetMy%20Pawn _asbp_patrolling_enemy))
  (AI|Components|Blackboard|SetValueasBool _returnvalue (Utilities|Name|MakeLiteralName "PathLooping") (Variables|/Game/Blueprints/AI/BP_PatrolPath.BP_PatrolPath_C|GetisLooping (Variables|/Game/Blueprints/AI/BP_Patrolling_Enemy.BP_Patrolling_Enemy_C|GetPatrol_Path _output_get)))
  (Class|BlackboardComponent|SetValueasInt _returnvalue (Utilities|Name|MakeLiteralName "Direction") 1)
  (AI|Components|Blackboard|SetValueasFloat (AI|GetBlackboard 0) (Utilities|Name|MakeLiteralName "WaitTime") (Variables|/Game/Blueprints/AI/BP_PatrolPath.BP_PatrolPath_C|GetTime%20Between%20Points (Variables|/Game/Blueprints/AI/BP_Patrolling_Enemy.BP_Patrolling_Enemy_C|GetPatrol_Path (Variables|Default|GetMy%20Pawn)))))

(fn ConstructionScript)