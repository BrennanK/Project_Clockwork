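; BP_Avatar is the player avatar Blueprint, handling punch collision spheres and rail grinding.
; The construction script snaps the spheres to hand sockets and, with BeginPlay, assigns component references such as camera, mesh and teleport effect.
; RailCollider overlaps store the other actor's spline and call BeginGrind if not already grinding.
; The punch collision event sets both spheres to PhysicsOnly whether punching or not.
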(event OnComponentBeginOverlap(RailCollider)
  (params (OverlappedComponent :type Primitive%20Component%20Object%20Reference) (OtherActor :type Actor%20Object%20Reference) (OtherComp :type Primitive%20Component%20Object%20Reference) (OtherBodyIndex :type Integer) (bFromSweep :type Boolean) (SweepResult :type Hit%20Result%20Structure%20%28by%20ref%29))
  (bind _returnvalue (Actor|GetComponentbyClass OtherActor "/Script/Engine.SplineComponent"))
  (if (== (Utilities|GetClass _returnvalue) "/Script/Engine.SplineComponent")
    (Variables|Default|SetourSpline _returnvalue)
    (if (not (Variables|Default|GetisGrinding))
      (Class|Avatar|BeginGrind)
      (Variables|Default|SetisGrinding true))))

(event EventBeginPlay
  (Variables|Default|SetplayerCamera (Variables|Default|GetCamera))
  (Variables|Default|SetisPunching false)
  (Variables|Default|SetcapsuleA (Variables|Default|GetCapsuleComponent)))

(event EventTick
  (params (DeltaSeconds :type Float%20%28single-precision%29)))

(event EventEnableandDisableCollision
  (bind _lefthandsphere (Variables|Default|GetleftHandSphere))
  (if (Variables|Default|GetisPunching)
    (Collision|SetCollisionEnabled _lefthandsphere "PhysicsOnly")
    (else
      (Collision|SetCollisionEnabled _lefthandsphere "PhysicsOnly"))))

(fn ConstructionScript
  (bind _mesh (Variables|Character|GetMesh))
  (Transformation|AttachComponentToComponent (Variables|Default|GetleftHandSphere) _mesh "hand_l" "SnapToTarget" "KeepWorld" "KeepWorld" true)
  (Transformation|AttachComponentToComponent (Variables|Default|GetrightHandSphere) _mesh "hand_r" "SnapToTarget" "KeepWorld" "KeepWorld" true)
  (Variables|Default|Setskeleton (Variables|Character|GetMesh))
  (Variables|Default|SetteleportationParticle (Variables|Default|GetTeleporter%20effect))
  (Variables|Default|SetcameraBoom (Variables|Default|GetCamera%20Boom)))