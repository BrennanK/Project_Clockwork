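; BP_NPC_HUD is a HUD Blueprint that draws a circular health meter for the player's BP_Avatar, despite the NPC name.
; BeginPlay creates a green dynamic instance of Circular_Health_Mat and caches the player character as BP_Avatar.
; Each DrawHUD call sets the material's Decimal parameter to current over max health, then draws it with DrawMaterialSimple at a fixed screen position and size.
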(event EventBeginPlay
  (bind _returnvalue (Rendering|Material|CreateDynamicMaterialInstance "/Game/Self_Materials/Materials/Circular_Health_Mat.Circular_Health_Mat" "None" :!class /Script/Engine.KismetMaterialLibrary))
  (Rendering|Material|SetVectorParameterValue _returnvalue "Color" "(R=0.004775,G=0.916667,B=0.063494,A=1.000000)" :!class /Script/Engine.MaterialInstanceDynamic)
  (bind _asbp_avatar (Utilities|Casting|CastToBP_Avatar (Game|GetPlayerCharacter 0)))
  (Rendering|Material|SetScalarParameterValue _returnvalue "Decimal" (/ (Variables|/Script/Book_Project.Avatar|GetcurrentHealth _asbp_avatar) (Variables|/Script/Book_Project.Avatar|GetmaxHealth _asbp_avatar)) :!class /Script/Engine.MaterialInstanceDynamic))

(event Collision|EventActorBeginOverlap
  (params (OtherActor :type Actor%20Object%20Reference)))

(event EventTick
  (params (DeltaSeconds :type Float%20%28single-precision%29)))

(event EventDrawHUD
  (params (SizeX :type Integer) (SizeY :type Integer))
  (Rendering|Material|SetScalarParameterValue (stale EventBeginPlay _returnvalue) "Decimal" (/ (Variables|/Script/Book_Project.Avatar|GetcurrentHealth (stale EventBeginPlay _asbp_avatar)) (Variables|/Script/Book_Project.Avatar|GetmaxHealth (stale EventBeginPlay _asbp_avatar))) :!class /Script/Engine.MaterialInstanceDynamic)
  (Class|HUD|DrawMaterialSimple (HUD|GetHUD (Game|GetPlayerController 0)) (stale EventBeginPlay _returnvalue) 9.5e+02 4.5e+02 1e+02 1e+02 1.0 false))

(fn ConstructionScript)