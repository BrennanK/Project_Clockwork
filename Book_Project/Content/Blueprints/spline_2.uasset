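; Spline-based rail actor that builds a repeated pillar-frame mesh along its Rail spline.
; The construction script divides the spline length by Spacer and adds a collidable, Z-forward spline mesh for each segment.
; Segment ends and tangents are sampled from the spline, with tangents scaled by TangentControl.
; A player pawn overlap on Rail only prints a debug string.
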(event OnComponentBeginOverlap(Rail)
  (params (OverlappedComponent :type Primitive%20Component%20Object%20Reference) (OtherActor :type Actor%20Object%20Reference) (OtherComp :type Primitive%20Component%20Object%20Reference) (OtherBodyIndex :type Integer) (bFromSweep :type Boolean) (SweepResult :type Hit%20Result%20Structure%20%28by%20ref%29))
  (if (== OtherActor (Game|Player|GetPlayerPawn 0))
    (Development|PrintString "We fixed the bastich")))

(event EventBeginPlay)

(event Collision|EventActorBeginOverlap
  (params (OtherActor :type Actor%20Object%20Reference)))

(event EventTick
  (params (DeltaSeconds :type Float%20%28single-precision%29)))

(fn ConstructionScript
  (bind _spacer (Variables|Default|GetSpacer))
  (bind _defaultsceneroot (Variables|Default|GetDefaultSceneRoot))
  (bind _tangentcontrol (Variables|Default|GetTangentControl))
  (bind _returnvalue (Transformation|GetWorldLocation _defaultsceneroot))
  (for _index (range 0 (.ReturnValue (Math|Float|Division(WholeandRemainder) (Spline|GetSplineLength (Variables|Default|GetRail)) _spacer)))
    (bind _returnvalue_2 (AddComponent|AddSplineMeshComponent false))
    (Components|StaticMesh|SetStaticMesh _returnvalue_2 "/Game/StarterContent/Props/SM_PillarFrame300.SM_PillarFrame300")
    (SplineMesh|SetForwardAxis _returnvalue_2 "Z" true)
    (Collision|SetCollisionEnabled _returnvalue_2 "QueryAndPhysics")
    (SplineMesh|SetStartandEnd _returnvalue_2 (- (Spline|GetLocationatDistanceAlongSpline (Variables|Default|GetRail) (* _index _spacer) "World") _returnvalue) (* (Spline|GetDirectionatDistanceAlongSpline (Variables|Default|GetRail) (* _index _spacer) "Local") _tangentcontrol) (- (Spline|GetLocationatDistanceAlongSpline (Variables|Default|GetRail) (+ _spacer (* _index _spacer)) "World") _returnvalue) (* (Spline|GetDirectionatDistanceAlongSpline (Variables|Default|GetRail) (+ _spacer (* _index _spacer)) "Local") _tangentcontrol) true :!class /Script/Engine.SplineMeshComponent)))