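; BP_Fire_Trap is an interactable obstacle Blueprint whose visible logic handles the fire trap's sound effects.
; Custom events start and stop the fire sound component.
; A water sound event passes an index to a function that sets the matching WaterSounds entry on the water audio component and plays it.
; Nothing in this graph calls these events, and BeginPlay, overlap, Tick and the construction script are empty.
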(event EventBeginPlay)

(event Collision|EventActorBeginOverlap
  (params (OtherActor :type Actor%20Object%20Reference)))

(event EventTick
  (params (DeltaSeconds :type Float%20%28single-precision%29)))

(event EventTurnonFireSound
  (Audio|Components|Audio|Play (Variables|Default|GetFire%20Sound%20Component) 0.0))

(event EventTurnOffFireSound
  (Audio|Components|Audio|Stop (Variables|Default|GetFire%20Sound%20Component)))

(event EventPlayWaterSoundEffect
  (params (indexOfSound :type Integer))
  (CallFunction|PlayWaterSoundsViaIndex indexOfSound))

(fn ConstructionScript)

(fn PlayWaterSoundsViaIndex
  (params (Index%20Of%20Sound :type Integer))
  (bind _water_sound_component (Variables|Default|GetWater%20Sound%20Component))
  (Audio|Components|Audio|SetSound _water_sound_component (Utilities|Array|Get(acopy) (Variables|Default|GetWater%20Sounds) Index%20Of%20Sound))
  (Audio|Components|Audio|Play _water_sound_component 0.0))