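; Puzzle block switch controller that shows a door-opening sequence by moving the view between the player avatar and a CameraMan camera.
; ChangeCameraPerspective toggles the blended view: going out it stuns the avatar, plays the opening sound, waits for it to finish, then calls BeginLerpingProcess; coming back it restores the avatar to normal after the blend.
; PlayMovingDoorSound plays an indexed door sound on the same audio component.
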(event EventBeginPlay)

(event Collision|EventActorBeginOverlap
  (params (OtherActor :type Actor%20Object%20Reference)))

(event EventTick
  (params (DeltaSeconds :type Float%20%28single-precision%29)))

(event EventChangeCameraPerspective
  (bind _audio (Variables|Default|GetAudio))
  (bind _timetotransitioncamera (Variables|Default|GettimeToTransitionCamera))
  (if (Variables|Default|GetperspectiveOnPlayer)
    (bind _asbp_avatar (Utilities|Casting|CastToBP_Avatar (Game|GetPlayerCharacter 0)))
    (Game|Player|SetViewTargetwithBlend (Game|GetPlayerController 0) _asbp_avatar _timetotransitioncamera "VTBlend_Linear" 0.0 false)
    (Utilities|FlowControl|Delay _timetotransitioncamera)
    (Variables|Default|SetperspectiveOnPlayer false)
    (Variables|/Script/Book_Project.Avatar|SetcurrentState _asbp_avatar "NORMAL")
    (else
      (bind _asbp_avatar_2 (Utilities|Casting|CastToBP_Avatar (Game|GetPlayerCharacter 0)))
      (Variables|/Script/Book_Project.Avatar|SetcurrentState _asbp_avatar_2 "STUNNED")
      (Game|Player|SetViewTargetwithBlend (Game|GetPlayerController 0) (Variables|Default|GetcameraMan) _timetotransitioncamera "VTBlend_Linear" 0.0 false)
      (Variables|Default|SetperspectiveOnPlayer true)
      (Utilities|FlowControl|Delay _timetotransitioncamera)
      (Audio|Components|Audio|SetSound _audio "/Game/StarterContent/Audio/Externally_Imported_Sounds/Door_Opening_Sound.Door_Opening_Sound")
      (Audio|Components|Audio|Play _audio 0.0)
      (Utilities|FlowControl|Delay (Variables|/Script/Engine.SoundBase|GetDuration (Variables|/Script/Engine.AudioComponent|GetSound _audio)))
      (Class|BlockSwitchController01|BeginLerpingProcess))))

(event EventPlayMovingDoorSound
  (params (index :type Integer))
  (bind _audio (Variables|Default|GetAudio))
  (Audio|Components|Audio|SetSound _audio (Utilities|Array|Get(acopy) (Variables|Default|GetDoor%20sounds) index))
  (Audio|Components|Audio|Play _audio 0.0))

(fn ConstructionScript)