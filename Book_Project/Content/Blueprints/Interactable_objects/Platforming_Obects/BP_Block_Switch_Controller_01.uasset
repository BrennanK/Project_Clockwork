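; Block switch controller for platforming puzzles that toggles the view between the player avatar and a CameraMan target.
; ChangeCameraPerspective stuns the avatar, blends the view to CameraMan, waits out the transition, then calls BeginLerpingProcess.
; When next triggered, it blends back to the avatar and restores its NORMAL state after the transition.
; The PerspectiveOnPlayer flag selects the branch and, despite its name, is true while CameraMan holds the view.
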(event EventBeginPlay)

(event Collision|EventActorBeginOverlap
  (params (OtherActor :type Actor%20Object%20Reference)))

(event EventTick
  (params (DeltaSeconds :type Float%20%28single-precision%29)))

(event EventChangeCameraPerspective
  (bind _camera_transition_time (Variables|Default|GetCamera%20Transition%20Time))
  (if (Variables|Default|GetperspectiveOnPlayer)
    (bind _asbp_avatar (Utilities|Casting|CastToBP_Avatar (Game|GetPlayerCharacter 0)))
    (Game|Player|SetViewTargetwithBlend (Game|GetPlayerController 0) _asbp_avatar _camera_transition_time "VTBlend_Linear" 0.0 false)
    (Utilities|FlowControl|Delay _camera_transition_time)
    (Variables|Default|SetperspectiveOnPlayer false)
    (Variables|/Script/Book_Project.Avatar|SetcurrentState _asbp_avatar "NORMAL")
    (else
      (bind _asbp_avatar_2 (Utilities|Casting|CastToBP_Avatar (Game|GetPlayerCharacter 0)))
      (Variables|/Script/Book_Project.Avatar|SetcurrentState _asbp_avatar_2 "STUNNED")
      (Game|Player|SetViewTargetwithBlend (Game|GetPlayerController 0) (Variables|Default|GetcameraMan) _camera_transition_time "VTBlend_Linear" 0.0 false)
      (Variables|Default|SetperspectiveOnPlayer true)
      (Utilities|FlowControl|Delay _camera_transition_time)
      (Class|BlockSwitchController01|BeginLerpingProcess))))

(fn ConstructionScript)